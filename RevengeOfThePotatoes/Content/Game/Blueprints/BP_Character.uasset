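; BP_Character is a player character with a sprite that walks left and right along the world Y axis.
; On BeginPlay it prints a debug string and adds the IMC_Input mapping context through BP_PlayerController's Enhanced Input subsystem.
; IA_Walk feeds movement input along Y.
; Each Tick turns the sprite's yaw to match the sign of Y velocity, keeping the last facing when stopped.
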(event Custom|UpdatePlayerRotation
  (bind _sprite (Variables|Default|GetSprite))
  (bind _relativerotation (Variables|/Script/Engine.SceneComponent|GetRelativeRotation _sprite))
  (Math|Float|CompareFloat (.y (Variables|/Script/Engine.MovementComponent|GetVelocity (Variables|Character|GetCharacterMovement))) 0.0
    (:>
      (Transformation|SetRelativeRotation _sprite (Math|Rotator|MakeRotator (.roll _relativerotation) (.pitch _relativerotation) 9e+01) false false))
    (:<
      (Transformation|SetRelativeRotation _sprite (Math|Rotator|MakeRotator (.roll _relativerotation) (.pitch _relativerotation) -9e+01) false false))))

(event Input|EnhancedActionEvents|EnhancedInputActionIA_Walk
  (params (ActionValue :type Float%20%28double-precision%29) (ElapsedSeconds :type Float%20%28double-precision%29) (TriggeredSeconds :type Float%20%28double-precision%29) (InputAction :type Input%20Action%20Object%20Reference :default "/Game/Game/Blueprints/Input/IA_Walk.IA_Walk"))
  (:Triggered
    (Pawn|Input|AddMovementInput "0.000000,1.000000,0.000000" ActionValue false)))

(event EventBeginPlay
  (Development|PrintString "Character")
  (bind _asbp_player_controller (Utilities|Casting|CastToBP_PlayerController (Game|GetPlayerController 0)))
  (Utilities|IsValid (PlayerController|LocalPlayerSubsystems|GetEnhancedInputLocalPlayerSubsystem _asbp_player_controller)
    (:Is%20Valid
      (Input|AddMappingContext (PlayerController|LocalPlayerSubsystems|GetEnhancedInputLocalPlayerSubsystem _asbp_player_controller) "/Game/Game/Blueprints/Input/IMC_Input.IMC_Input" 0 "(bIgnoreAllPressedKeysUntilRelease=True,bForceImmediately=False)"))))

(event EventTick
  (params (DeltaSeconds :type Float%20%28single-precision%29))
  (CallFunction|UpdatePlayerRotation))

(fn ConstructionScript)