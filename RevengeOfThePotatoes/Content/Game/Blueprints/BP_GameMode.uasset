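; Game mode that populates the level with potato and carrot characters when play begins.
; It finds every BP_SpawnPoint and branches on its CharacterType, spawning a batch of potato characters or a single carrot character there.
; Each spawn gets a small random X/Y offset from the point and always spawns, adjusting position to avoid collisions where possible.
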(event EventBeginPlay
  (bind _outactors (Actor|GetAllActorsOfClass "/Game/Game/Blueprints/BP_SpawnPoint.BP_SpawnPoint_C"))
  (for _array_element _outactors
    (switch Utilities|FlowControl|Switch|SwitchonE_CharacterType (Variables|/Game/Game/Blueprints/BP_SpawnPoint.BP_SpawnPoint_C|GetCharacterType _array_element)
      (:NewEnumerator0
        (for _index (range 0 5)
          (Game|SpawnActorfromClass "/Game/Game/Characters/BPC_PotatoCharacter.BPC_PotatoCharacter_C" (Math|Transform|MakeTransform (Math|Vector|MakeVector (+ (.x (.location (Transformation|GetActorTransform _array_element))) (Math|Random|RandomFloatinRange -5e+01 5e+01)) (+ (.y (.location (Transformation|GetActorTransform _array_element))) (Math|Random|RandomFloatinRange -1e+01 1e+01)) (.z (.location (Transformation|GetActorTransform _array_element)))) (.rotation (Transformation|GetActorTransform _array_element)) (.scale (Transformation|GetActorTransform _array_element))) "AdjustIfPossibleButAlwaysSpawn" "MultiplyWithRoot" 0 0)))
      (:NewEnumerator1
        (Game|SpawnActorfromClass "/Game/Game/Characters/BPC_CarrotCharacter.BPC_CarrotCharacter_C" (Math|Transform|MakeTransform (Math|Vector|MakeVector (+ (.x (.location (Transformation|GetActorTransform _array_element))) (Math|Random|RandomFloatinRange -5e+01 5e+01)) (+ (.y (.location (Transformation|GetActorTransform _array_element))) (Math|Random|RandomFloatinRange -1e+01 1e+01)) (.z (.location (Transformation|GetActorTransform _array_element)))) (.rotation (Transformation|GetActorTransform _array_element)) (.scale (Transformation|GetActorTransform _array_element))) "AdjustIfPossibleButAlwaysSpawn" "MultiplyWithRoot" 0 0)))))

(fn ConstructionScript)