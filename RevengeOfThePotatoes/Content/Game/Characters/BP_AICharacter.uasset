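; AI-controlled character with a sprite that detects and walks toward characters of a different CharacterType.
; When PawnSensing sees another BP_AICharacter of a differing type, it stores that pawn and issues an AI MoveTo toward it.
; Each tick the sprite's relative yaw flips between 90 and -90 degrees based on the sign of Y velocity, so it faces the direction of movement.
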(event OnSeePawn(PawnSensing)
  (params (Pawn :type Pawn%20Object%20Reference))
  ;[1 1 1] Walk towards other pawn
  (bind _asbp_aicharacter (Utilities|Casting|CastToBP_AICharacter Pawn))
  (if (Utilities|Enum|NotEqual(Enum) (Variables|BP_AICharacter_C|GetCharacterType _asbp_aicharacter) (Variables|Default|GetCharacterType))
    (Variables|Default|SetisSeeingPlayer? true)
    (Variables|Default|SetPawnSeen Pawn)
    (CallFunction|FollowPlayer)))

(event Custom|UpdatePlayerRotation
  (bind _sprite (Variables|Default|GetSprite))
  (bind _relativerotation (Variables|/Script/Engine.SceneComponent|GetRelativeRotation _sprite))
  ;[1 1 1] Rotate sprite according to character rotation
  (Math|Float|CompareFloat (.y (Variables|/Script/Engine.MovementComponent|GetVelocity (Variables|Character|GetCharacterMovement))) 0.0
    (:>
      (Transformation|SetRelativeRotation _sprite (Math|Rotator|MakeRotator (.roll _relativerotation) (.pitch _relativerotation) 9e+01) false false))
    (:<
      (Transformation|SetRelativeRotation _sprite (Math|Rotator|MakeRotator (.roll _relativerotation) (.pitch _relativerotation) -9e+01) false false))))

(event Custom|FollowPlayer
  ;[1 1 1] Walk towards other pawn
  (if (Variables|Default|GetisSeeingPlayer?)
    (AI|AIMoveTo self "0, 0, 0" (Variables|Default|GetPawnSeen) 5.0 false)))

(event EventTick
  (params (DeltaSeconds :type Float%20%28single-precision%29))
  ;[1 1 1] Rotate sprite according to character rotation
  (CallFunction|UpdatePlayerRotation))

(fn ConstructionScript)